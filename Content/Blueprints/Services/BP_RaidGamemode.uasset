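; Raid game mode that spawns basic enemy bots and reacts to actor kills.
; SpawnNewBot runs an EQS query for a spawn location and spawns BP_BasicEnemy at each returned point, with debug spheres and name prints.
; BeginPlay binds the actor-killed event, whose handler calls RestartPlayerAtPlayerStart using the killer pawn as the start spot, with no player controller supplied.
; Nothing in this graph calls SpawnNewBot.
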(event `self.SpawnNewBot`
  (bind _returnvalue (`EnvQueryManager.RunEQSQuery` "/Game/Blueprints/InGameAssets/AI/EQS_FindSpawnLocation.EQS_FindSpawnLocation" self "RandomBest25Pct"))
  (add `EnvQueryInstanceBlueprintWrapper.OnQueryFinishedEvent` _returnvalue (delegate `OnQueryFinishedEvent_Event_0`)))

(event `OnQueryFinishedEvent_Event_0`
  (params (QueryInstance :type "EnvQueryInstanceBlueprintWrapper Object Reference") (QueryStatus :type "EEnvQueryStatus Enum" :default "Processing"))
  (switch `EEnvQueryStatus` QueryStatus
    (:`Success`
      (bind _resultlocations (`EnvQueryInstanceBlueprintWrapper.GetQueryResultsAsLocations` QueryInstance))
      (for _array_element _resultlocations
        (`KismetSystemLibrary.DrawDebugSphere` _array_element 50.0 12 (struct :`R` 1.0 :`G` 0.783492 :`A` 1.0) 2.0 5.0)
        (bind _returnvalue (`|SpawnActorFromClass` "/Game/Blueprints/InGameAssets/AI/AutonomicDevices/BP_BasicEnemy.BP_BasicEnemy_C" (`KismetMathLibrary.MakeTransform` _array_element) "AdjustIfPossibleButDontSpawnIfColliding" "OverrideRootScale" null null))
        (`KismetSystemLibrary.PrintString` (`KismetSystemLibrary.GetDisplayName` _returnvalue))))))

(event `self.ReceiveBeginPlay`
  (add `self.m_onActorKilled` (delegate `m_onActorKilled_Event`)))

(event `m_onActorKilled_Event` :!signature `self.m_onActorKilled`
  (params (victimActor :type "Actor Object Reference") (killerActor :type "Actor Object Reference") (killerController :type "Controller Object Reference"))
  (bind _aspawn (cast `Pawn` killerActor))
  (`self.RestartPlayerAtPlayerStart` null _aspawn))

(fn `UserConstructionScript`)